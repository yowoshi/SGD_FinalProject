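; Game mode that holds carry state and score for a food-carrying game and manages its HUD widgets.
; BeginPlay resets carry flags and counters, creates the food-type and Press E widgets, and displays the score widget.
; Tick polls the carry flags to add or remove the food type A or B indicator.
; AddTargetPoints updates Score, while pause-and-main-menu logic is left unconnected.
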(event Custom|AddTargetPoints
  (params (Score :type Integer))
  ;[1 0.5358 0.4337] Sets and Increases Score
  (Variables|Default|SetScore (+ Score (Variables|Default|GetScore))))

(event EventTick
  (params (DeltaSeconds :type Float%20%28single-precision%29))
  ;[1 0.5591 0.8105] Checks for FoodTypeA Widget
  (if (and (Variables|Default|GetisFoodTypeA) (Variables|Default|GetisCarrying))
    (if (not (Variables|Default|GetisShowingFoodTypeA))
      (UserInterface|Viewport|AddtoViewport (Variables|Default|GetShowFoodTypeAWidget) 0)
      (Variables|Default|SetisShowingFoodTypeA true))
    (else
      (Widget|RemovefromParent (Variables|Default|GetShowFoodTypeAWidget))
      (Variables|Default|SetisShowingFoodTypeA false)
      ;[0.7534 1 0.6146] Checks for FoodTypeB Widget
      (if (Variables|Default|GetisCarrying)
        (if (not (Variables|Default|GetisShowingFoodTypeB))
          (UserInterface|Viewport|AddtoViewport (Variables|Default|GetShowFoodTypeBWidget) 0)
          (Variables|Default|SetisShowingFoodTypeB true))
        (else
          (Widget|RemovefromParent (Variables|Default|GetShowFoodTypeBWidget))
          (Variables|Default|SetisShowingFoodTypeB false))))))

(event EventBeginPlay
  ;[0.5335 0.8605 1] Sets Variables and Widgets
  (Variables|Default|SetisCarrying false)
  (Variables|Default|SetisGrabbing false)
  (Variables|Default|SetisFoodTypeA false)
  (Variables|Default|SetCountA 0)
  (Variables|Default|SetCountB 0)
  (bind _returnvalue (UserInterface|CreateWidget "/Game/Widgets/W_isCarryingFoodTypeA.W_isCarryingFoodTypeA_C"))
  (Variables|Default|SetShowFoodTypeAWidget _returnvalue)
  (bind _returnvalue_2 (UserInterface|CreateWidget "/Game/Widgets/W_isCarryingFoodTypeB.W_isCarryingFoodTypeB_C"))
  (Variables|Default|SetShowFoodTypeBWidget _returnvalue_2)
  (bind _returnvalue_3 (UserInterface|CreateWidget "/Game/Widgets/W_Press_E.W_Press_E_C"))
  (Variables|Default|SetPressE _returnvalue_3)
  (bind _returnvalue_4 (UserInterface|CreateWidget "/Game/Widgets/W_Score.W_Score_C"))
  (UserInterface|Viewport|AddtoViewport _returnvalue_4 0))

(fn ConstructionScript)