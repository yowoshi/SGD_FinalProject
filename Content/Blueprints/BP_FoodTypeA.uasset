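; BP_FoodTypeA is a food pickup actor that the player grabs when nearby.
; Each tick it measures distance to the player pawn, showing or hiding a W_Press_E prompt created on BeginPlay.
; When BP_GameModeBase.IsGrabbing is set within range, it destroys itself, plays the grab sound and removes the prompt.
; It also sets IsCarrying and IsFoodTypeA on the game mode, which holds the shared carry state.
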(event EventBeginPlay
  ;[1 1 1] Creates Widget and Variable
  (bind _returnvalue (UserInterface|CreateWidget "/Game/Widgets/W_Press_E.W_Press_E_C"))
  (Variables|Default|SetPress%20E _returnvalue))

(event EventTick
  (params (DeltaSeconds :type Float%20%28single-precision%29))
  (bind _returnvalue (Game|Player|GetPlayerPawn 0))
  (bind _returnvalue_2 (Transformation|GetActorLocation))
  (bind _returnvalue_3 (Game|GetGameMode))
  (bind _returnvalue_4 (Transformation|GetActorLocation _returnvalue))
  (bind _returnvalue_5 (Math|Vector|Distance(Vector) _returnvalue_2 _returnvalue_4))
  (bind _returnvalue_6 (<= _returnvalue_5 1.5e+02))
  ;[1 1 1] Checks Location and Destroys Actor when Pressing E
  (bind _asbp_game_mode_base (Utilities|Casting|CastToBP_GameModeBase _returnvalue_3))
  (if (and (Variables|/Game/Blueprints/BP_GameModeBase.BP_GameModeBase_C|GetisGrabbing _asbp_game_mode_base) _returnvalue_6)
    (Actor|DestroyActor)
    (Audio|PlaySound2D "/Game/SoundEffects/Grab.Grab" 1.0 1.0 0.0 0 0)
    (bind _asbp_game_mode_base_2 (Utilities|Casting|CastToBP_GameModeBase _returnvalue_3))
    (Variables|/Game/Blueprints/BP_GameModeBase.BP_GameModeBase_C|SetisCarrying _asbp_game_mode_base_2 true)
    (Variables|/Game/Blueprints/BP_GameModeBase.BP_GameModeBase_C|SetisFoodTypeA _asbp_game_mode_base_2 true)
    (if (Variables|/Game/Blueprints/BP_GameModeBase.BP_GameModeBase_C|GetisCarrying _asbp_game_mode_base)
      (Widget|RemovefromParent (Variables|Default|GetPress%20E))
      (Variables|Default|SetisShowingPressE false))
    (elif _returnvalue_6
      ;[1 1 1] Creates Press E Widget
      (if (not (Variables|Default|GetisShowingPressE))
        (UserInterface|Viewport|AddtoViewport (Variables|Default|GetPress%20E) 0)
        (Variables|Default|SetisShowingPressE true))
      (else
        (Widget|RemovefromParent (Variables|Default|GetPress%20E))
        (Variables|Default|SetisShowingPressE false)))))

(fn ConstructionScript)