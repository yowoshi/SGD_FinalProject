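; Spawner actor that places BP_FoodTypeB pickups at random reachable navmesh points around itself, slightly raised off the ground.
; BeginPlay spawns one nearby without counting it.
; Tick checks the game mode's CountB and, while below three, uses a Delay to spawn another in a much wider radius every ten seconds or so.
; Each delayed spawn increments CountB and prints it; nothing here decrements it.
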(event EventTick
  (params (DeltaSeconds :type Float%20%28single-precision%29))
  (bind _asbp_game_mode_base (Utilities|Casting|CastToBP_GameModeBase (Game|GetGameMode)))
  (if (< (Variables|/Game/Blueprints/BP_GameModeBase.BP_GameModeBase_C|GetCountB _asbp_game_mode_base) 3)
    (Utilities|FlowControl|Delay 1e+01)
    (Game|SpawnActorfromClass "/Game/Blueprints/BP_FoodTypeB.BP_FoodTypeB_C" (Math|Conversions|ToTransform(Vector) (+ (.RandomLocation (AI|Navigation|GetRandomReachablePointinRadius (Transformation|GetActorLocation) 2e+04 0 0)) "0, 0,50.000000")) "Undefined" 0 0)
    (Variables|/Game/Blueprints/BP_GameModeBase.BP_GameModeBase_C|SetCountB _asbp_game_mode_base (+ (Variables|/Game/Blueprints/BP_GameModeBase.BP_GameModeBase_C|GetCountB _asbp_game_mode_base) 1))
    (Development|PrintString (Utilities|String|ToString(Integer) (Variables|/Game/Blueprints/BP_GameModeBase.BP_GameModeBase_C|GetCountB _asbp_game_mode_base)))))

(event EventBeginPlay
  (Game|SpawnActorfromClass "/Game/Blueprints/BP_FoodTypeB.BP_FoodTypeB_C" (Math|Conversions|ToTransform(Vector) (+ (.RandomLocation (AI|Navigation|GetRandomReachablePointinRadius (Transformation|GetActorLocation) 1e+03 0 0)) "0, 0,50.000000")) "Undefined" 0 0))

(fn ConstructionScript)