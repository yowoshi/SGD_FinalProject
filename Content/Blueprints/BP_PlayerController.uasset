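; Player pawn (named as a controller, with a capsule) handling first-person-style movement, mouse look, pause menu and food carrying.
; Grab sets game mode flags and, when carrying, drops by spawning food type A or B ahead; movement slows while carrying.
; Tick starts or fades footstep audio from raw WASD key flags, stopping it when paused.
; Escape flip-flops the pause widget; the zookeeper overlap only casts, with no follow-up.
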(event OnComponentBeginOverlap(CapsuleComponent)
  (params (OverlappedComponent :type Primitive%20Component%20Object%20Reference) (OtherActor :type Actor%20Object%20Reference) (OtherComp :type Primitive%20Component%20Object%20Reference) (OtherBodyIndex :type Integer) (bFromSweep :type Boolean) (SweepResult :type Hit%20Result%20Structure%20%28by%20ref%29))
  (Utilities|Casting|CastToBP_ZooKeeper OtherActor))

(event EventTick
  (params (DeltaSeconds :type Float%20%28single-precision%29))
  ;[1 1 1] Checks if Audio Should be Playing
  (if (Game|IsGamePaused)
    (if (Variables|Default|GetisPlaying)
      (Audio|Components|Audio|Stop (Variables|Default|GetWalking)))
    (else
      (if (Math|Boolean|ORBoolean (Variables|Default|GetW) (Variables|Default|GetA) (Variables|Default|GetS) (Variables|Default|GetD))
        (Variables|Default|SetisShouldBePlaying true)
        (else
          (Variables|Default|SetisShouldBePlaying false)))
      (if (Variables|Default|GetisShouldBePlaying)
        (if (not (Variables|Default|GetisPlaying))
          (bind _returnvalue (Audio|SpawnSound2D "/Game/SoundEffects/Footstep.Footstep" 1.0 1.0 0.0 0))
          (Variables|Default|SetWalking _returnvalue)
          (Variables|Default|SetisPlaying true))
        (elif (Variables|Default|GetisPlaying)
          (Audio|Components|Audio|FadeOut (Variables|Default|GetWalking) 0.25 0.0 "Linear" :!class /Script/Engine.AudioComponent)
          (Variables|Default|SetisPlaying false))))))

(event EventBeginPlay
  ;[1 1 1] Checks if User is Inputting
  (Variables|Default|SetisPlaying false))

(event Input|ActionEvents|InputActionGrab
  (params (Key :type Key%20Structure :default "None"))
  (bind _returnvalue (Pawn|GetControlRotation :!class /Script/Engine.Pawn))
  (bind _returnvalue_2 (Transformation|GetActorLocation))
  (bind _returnvalue_3 (Game|GetGameMode))
  (bind _returnvalue_4 (Math|Vector|GetForwardVector _returnvalue))
  (bind _returnvalue_5 (* _returnvalue_4 1e+02))
  (bind _returnvalue_6 (+ _returnvalue_5 _returnvalue_2))
  (bind _returnvalue_7 (+ _returnvalue_6 "0, 0,-20.000000"))
  (bind _returnvalue_8 (Math|Conversions|ToTransform(Vector) _returnvalue_7))
  ;[1 1 1] Checks if Pressing E
  (:Pressed
    (bind _asbp_game_mode_base (Utilities|Casting|CastToBP_GameModeBase _returnvalue_3))
    (Variables|/Game/Blueprints/BP_GameModeBase.BP_GameModeBase_C|SetisGrabbing _asbp_game_mode_base true)
    ;[1 1 1] Grabbing Object from Class
    (bind _asbp_game_mode_base_2 (Utilities|Casting|CastToBP_GameModeBase (Game|GetGameMode)))
    (if (Variables|/Game/Blueprints/BP_GameModeBase.BP_GameModeBase_C|GetisCarrying _asbp_game_mode_base_2)
      ;[1 1 1] Dropping Object From Class
      (bind _asbp_game_mode_base_3 (Utilities|Casting|CastToBP_GameModeBase (Game|GetGameMode)))
      (Variables|/Game/Blueprints/BP_GameModeBase.BP_GameModeBase_C|SetisCarrying _asbp_game_mode_base_3 false)
      (Development|PrintString "Dropped")
      (if (Variables|/Game/Blueprints/BP_GameModeBase.BP_GameModeBase_C|GetisFoodTypeA _asbp_game_mode_base_3)
        (Audio|PlaySound2D "/Game/SoundEffects/Drop.Drop" 1.0 1.0 0.0 0 0)
        (Utilities|FlowControl|Delay 0.2)
        (Game|SpawnActorfromClass "/Game/Blueprints/BP_FoodTypeA.BP_FoodTypeA_C" _returnvalue_8 "Undefined" 0 0)
        (else
          (Audio|PlaySound2D "/Game/SoundEffects/Drop.Drop" 1.0 1.0 0.0 0 0)
          (Utilities|FlowControl|Delay 0.2)
          (Game|SpawnActorfromClass "/Game/Blueprints/BP_FoodTypeB.BP_FoodTypeB_C" _returnvalue_8 "Undefined" 0 0)))))
  (:Released
    (bind _asbp_game_mode_base_4 (Utilities|Casting|CastToBP_GameModeBase _returnvalue_3))
    (Variables|/Game/Blueprints/BP_GameModeBase.BP_GameModeBase_C|SetisGrabbing _asbp_game_mode_base_4 false)))

(event Input|KeyboardEvents|Escape
  (params (Key :type Key%20Structure :default "None"))
  (bind _returnvalue (Game|GetPlayerController 0))
  ;[1 1 1] Pause
  (:Pressed
    (Utilities|FlowControl|FlipFlop
      (:A
        (Variables|/Script/Engine.PlayerController|SetbShowMouseCursor _returnvalue true)
        (bind _returnvalue_2 (UserInterface|CreateWidget "/Game/Widgets/W_Pause.W_Pause_C"))
        (UserInterface|Viewport|AddtoViewport _returnvalue_2 0)
        (Game|SetGamePaused true))
      (:B
        (Variables|/Script/Engine.PlayerController|SetbShowMouseCursor _returnvalue false)
        (Widget|RemovefromParent _returnvalue_2)
        (Game|SetGamePaused false)))))

(event Input|KeyboardEvents|W
  (params (Key :type Key%20Structure :default "None"))
  ;[1 1 1] Checks if User is Inputting
  (:Pressed
    (Variables|Default|SetW true))
  (:Released
    (Variables|Default|SetW false)))

(event Input|KeyboardEvents|A
  (params (Key :type Key%20Structure :default "None"))
  ;[1 1 1] Checks if User is Inputting
  (:Pressed
    (Variables|Default|SetA true))
  (:Released
    (Variables|Default|SetA false)))

(event Input|KeyboardEvents|S
  (params (Key :type Key%20Structure :default "None"))
  ;[1 1 1] Checks if User is Inputting
  (:Pressed
    (Variables|Default|SetS true))
  (:Released
    (Variables|Default|SetS false)))

(event Input|KeyboardEvents|D
  (params (Key :type Key%20Structure :default "None"))
  ;[1 1 1] Checks if User is Inputting
  (:Pressed
    (Variables|Default|SetD true))
  (:Released
    (Variables|Default|SetD false)))

(event Input|AxisEvents|InputAxisMoveRight
  (params (AxisValue :type Float%20%28single-precision%29))
  (bind _returnvalue (Pawn|GetControlRotation :!class /Script/Engine.Pawn))
  (bind _returnvalue_2 (Math|Vector|GetRightVector _returnvalue))
  ;[1 1 1] Forward Movement + Tracks Location
  ;;[1 0.6071 0.5892] IsCarying = True
  (bind _asbp_game_mode_base (Utilities|Casting|CastToBP_GameModeBase (Game|GetGameMode)))
  (if (Variables|/Game/Blueprints/BP_GameModeBase.BP_GameModeBase_C|GetisCarrying _asbp_game_mode_base)
    (Pawn|Input|AddMovementInput (* _returnvalue_2 0.4) AxisValue false)
    (else
      ;;[0.8008 0.9781 1] IsCarying = False
      (Pawn|Input|AddMovementInput _returnvalue_2 AxisValue false))))

(event Input|AxisEvents|InputAxisMoveForward
  (params (AxisValue :type Float%20%28single-precision%29))
  (bind _returnvalue (Pawn|GetControlRotation :!class /Script/Engine.Pawn))
  (bind _returnvalue_2 (Math|Vector|GetForwardVector _returnvalue))
  ;[1 1 1] Forward Movement + Tracks Location
  ;;[1 0.4716 0.4018] IsCarrying = True
  (bind _asbp_game_mode_base (Utilities|Casting|CastToBP_GameModeBase (Game|GetGameMode)))
  (if (Variables|/Game/Blueprints/BP_GameModeBase.BP_GameModeBase_C|GetisCarrying _asbp_game_mode_base)
    (Pawn|Input|AddMovementInput (* _returnvalue_2 0.4) AxisValue false)
    (else
      ;;[0.7181 0.95 1] IsCarrying = False
      (Pawn|Input|AddMovementInput _returnvalue_2 AxisValue false))))

(event Input|AxisEvents|InputAxisLookUp
  (params (AxisValue :type Float%20%28single-precision%29))
  ;[1 1 1] Camera Follows Mouse
  (Pawn|Input|AddControllerPitchInput AxisValue))

(event Input|AxisEvents|InputAxisLookRight
  (params (AxisValue :type Float%20%28single-precision%29))
  ;[1 1 1] Camera Follows Mouse
  (Pawn|Input|AddControllerYawInput AxisValue))

(fn ConstructionScript)