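; BP_ZooKeeper is an enemy character that ends the game when its capsule overlaps the player pawn.
; The overlap plays the game-over sound, shows the W_GameOver widget, pauses the game and reveals the cursor.
; An unwired distance-based AI block would wander randomly or chase a nearby player faster, with timed boot-step sounds.
; Tick is empty, so that movement logic never runs here.
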(event OnComponentBeginOverlap(CapsuleComponent)
  (params (OverlappedComponent :type Primitive%20Component%20Object%20Reference) (OtherActor :type Actor%20Object%20Reference) (OtherComp :type Primitive%20Component%20Object%20Reference) (OtherBodyIndex :type Integer) (bFromSweep :type Boolean) (SweepResult :type Hit%20Result%20Structure%20%28by%20ref%29))
  ;[1 1 1] Ends Game on Collision
  (if (== OtherActor (Game|Player|GetPlayerPawn 0))
    (Audio|PlaySound2D "/Game/SoundEffects/GameOver.GameOver" 1.0 1.0 0.0 0 0)
    (bind _returnvalue (UserInterface|CreateWidget "/Game/Widgets/W_GameOver.W_GameOver_C"))
    (UserInterface|Viewport|AddtoViewport _returnvalue 0)
    (Game|SetGamePaused true)
    (Variables|/Script/Engine.PlayerController|SetbShowMouseCursor (Game|GetPlayerController 0) true)))

(event EventBeginPlay
  (Variables|Default|SetPlayingAudio false))

(event EventTick
  (params (DeltaSeconds :type Float%20%28single-precision%29)))

(fn ConstructionScript)