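; Food spawn manager Blueprint that periodically lowers two counters, CountA and CountB, on BP_GameModeBase.
; BeginPlay sets the StartSpawning flag after a two-minute delay.
; Tick then runs through a Delay, which works as a repeating timer that decrements both counters by one every 80 seconds.
; The Blueprint itself spawns no actors.
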(event EventBeginPlay
  (Utilities|FlowControl|Delay 1.2e+02)
  (Variables|Default|SetstartSpawning true))

(event EventTick
  (params (DeltaSeconds :type Float%20%28single-precision%29))
  (if (Variables|Default|GetstartSpawning)
    (Utilities|FlowControl|Delay 8e+01)
    (bind _asbp_game_mode_base (Utilities|Casting|CastToBP_GameModeBase (Game|GetGameMode)))
    (Variables|/Game/Blueprints/BP_GameModeBase.BP_GameModeBase_C|SetCountA _asbp_game_mode_base (- (Variables|/Game/Blueprints/BP_GameModeBase.BP_GameModeBase_C|GetCountA _asbp_game_mode_base) 1))
    (Variables|/Game/Blueprints/BP_GameModeBase.BP_GameModeBase_C|SetCountB _asbp_game_mode_base (- (Variables|/Game/Blueprints/BP_GameModeBase.BP_GameModeBase_C|GetCountB _asbp_game_mode_base) 1))))

(fn ConstructionScript)