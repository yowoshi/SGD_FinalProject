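; BP_ZookeeperSpawner is a placed actor that spawns AI-possessed BP_ZooKeeper characters at its own location as the player's score rises.
; BeginPlay spawns the first zookeeper with a default controller and resets the extra-spawn counter.
; Tick polls Score on BP_GameModeBase and spawns up to two more as successive thresholds are reached, using the counter and a flag so each fires once.
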(event EventTick
  (params (DeltaSeconds :type Float%20%28single-precision%29))
  ;[1 1 1] Spawns Zookeeper when Condition is Met
  (bind _asbp_game_mode_base (Utilities|Casting|CastToBP_GameModeBase (Game|GetGameMode)))
  (if (or (and (== (Variables|Default|GetNumber%20of%20Spawned%20Zookeepers) 0) (>= (Variables|/Game/Blueprints/BP_GameModeBase.BP_GameModeBase_C|GetScore _asbp_game_mode_base) 10)) (and (== (Variables|Default|GetNumber%20of%20Spawned%20Zookeepers) 1) (>= (Variables|/Game/Blueprints/BP_GameModeBase.BP_GameModeBase_C|GetScore _asbp_game_mode_base) 20)))
    (Variables|Default|SetSpawn%20a%20Zookeeper true))
  (if (Variables|Default|GetSpawn%20a%20Zookeeper)
    (bind _returnvalue (Game|SpawnActorfromClass "/Game/Blueprints/BP_ZooKeeper.BP_ZooKeeper_C" (Math|Conversions|ToTransform(Vector) (Transformation|GetWorldLocation (Variables|Default|GetDefaultSceneRoot))) "Undefined" 0 0))
    (Pawn|SpawnDefaultController _returnvalue)
    (Variables|Default|SetNumber%20of%20Spawned%20Zookeepers (+ (Variables|Default|GetNumber%20of%20Spawned%20Zookeepers) 1))
    (Variables|Default|SetSpawn%20a%20Zookeeper false)))

(event EventBeginPlay
  ;[1 1 1] Spawns Zookeeper at Begin Play
  (bind _returnvalue (Game|SpawnActorfromClass "/Game/Blueprints/BP_ZooKeeper.BP_ZooKeeper_C" (Math|Conversions|ToTransform(Vector) (Transformation|GetWorldLocation (Variables|Default|GetDefaultSceneRoot))) "Undefined" 0 0))
  (Pawn|SpawnDefaultController _returnvalue)
  (Variables|Default|SetNumber%20of%20Spawned%20Zookeepers 0))

(fn ConstructionScript)