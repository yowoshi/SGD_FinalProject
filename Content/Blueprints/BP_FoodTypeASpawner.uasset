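; Spawner actor that places BP_FoodTypeA actors at its root component's location.
; It spawns one on BeginPlay without incrementing the game mode's CountA.
; Tick checks that BP_GameModeBase's CountA is below a small cap, then uses a Delay to pace each further spawn.
; Each delayed spawn increments CountA and prints the new value.
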(event EventTick
  (params (DeltaSeconds :type Float%20%28single-precision%29))
  (bind _asbp_game_mode_base (Utilities|Casting|CastToBP_GameModeBase (Game|GetGameMode)))
  (if (< (Variables|/Game/Blueprints/BP_GameModeBase.BP_GameModeBase_C|GetCountA _asbp_game_mode_base) 3)
    (Utilities|FlowControl|Delay 1e+01)
    (Game|SpawnActorfromClass "/Game/Blueprints/BP_FoodTypeA.BP_FoodTypeA_C" (Math|Conversions|ToTransform(Vector) (Transformation|GetWorldLocation (Variables|Default|GetDefaultSceneRoot))) "Undefined" 0 0)
    (Variables|/Game/Blueprints/BP_GameModeBase.BP_GameModeBase_C|SetCountA _asbp_game_mode_base (+ (Variables|/Game/Blueprints/BP_GameModeBase.BP_GameModeBase_C|GetCountA _asbp_game_mode_base) 1))
    (Development|PrintString (Utilities|String|ToString(Integer) (Variables|/Game/Blueprints/BP_GameModeBase.BP_GameModeBase_C|GetCountA _asbp_game_mode_base)))))

(event EventBeginPlay
  (Game|SpawnActorfromClass "/Game/Blueprints/BP_FoodTypeA.BP_FoodTypeA_C" (Math|Conversions|ToTransform(Vector) (Transformation|GetWorldLocation (Variables|Default|GetDefaultSceneRoot))) "Undefined" 0 0))

(fn ConstructionScript)